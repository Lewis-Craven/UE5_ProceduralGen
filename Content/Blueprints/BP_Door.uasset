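; Interactive door that the player can open, close, lock with a key, and destroy through damage.
; Interact toggles timelines that swing the door away from the player via a camera dot product, slide it sideways, or raise it.
; Forward and backward overlap volumes show that side's open and lock billboard prompts.
; The construction script applies lock material, optional light, and Regular or Heavy health, swing speed and frame material.
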(event `self.ReceiveBeginPlay`
  ;[1 1 1] Sets The Speed of The Door Opening
  (`TimelineComponent.SetPlayRate` (`self.Door Open Timeline`) (`self.DoorOpenSpeed`))
  (set `self.CurrentHealth` (`self.MaxHealth`))
  (`SceneComponent.SetVisibility` (`self.OpenDoorBillboardForward`) false false)
  (`SceneComponent.SetVisibility` (`self.OpenDoorBillboardBackward`) false false)
  (`SceneComponent.SetVisibility` (`self.LockDoorBillboardBackward`) false false)
  (`SceneComponent.SetVisibility` (`self.LockDoorBillboardForward`) false false)
  ; Use Later to Add door collission
  (if (`self.IsLocked`)
    _))

(event `/Game/Blueprints/BPI_Interact.Interact`
  (bind _opendoorbillboardforward (`self.OpenDoorBillboardForward`))
  ;[1 1 1] Open Door Interaction
  (if (not (`self.IsDestroyed`))
    ;;[1 1 1] Checks If Door Is Locked
    (if (not (`self.IsLocked`))
      (`/Engine/EditorBlueprintResources/StandardMacros.FlipFlop`
        (:`A`
          (`BillboardComponent.SetSprite` _opendoorbillboardforward "/Game/Blueprints/T_CLOSE.T_CLOSE")
          (`BillboardComponent.SetSprite` (`self.OpenDoorBillboardBackward`) "/Game/Blueprints/T_CLOSE.T_CLOSE")
          (`AudioComponent.Play` (`self.PIXABAYdoor-open-close_OPEN`) 0.0)
          (switch `/Game/Blueprints/ENums/E_DoorRotationType` (`self.RotateType`)
            (:`NewEnumerator0`
              ;;[1 1 1] Gets player position to determine which side of the door they are on
              (bind _asbp_first_person_character (cast `/Game/FirstPerson/Blueprints/BP_FirstPersonCharacter` (`GameplayStatics.GetPlayerCharacter` 0)))
              (`/Engine/EditorBlueprintResources/StandardMacros.CompareFloat` (`KismetMathLibrary.Dot_VectorVector` (`SceneComponent.GetForwardVector` (`self.Arrow`)) (`SceneComponent.GetForwardVector` (`/Game/FirstPerson/Blueprints/BP_FirstPersonCharacter.FirstPersonCamera` _asbp_first_person_character)))
                (:`>`
                  (set `self.RotateDirection` (struct :`Yaw` 90.0))
                  ;;[1 1 1] Opens the door
                  (bind (_direction _newtrack_1) (`Timeline|Door Open Timeline` :!label _label)
                    (:`Update`
                      (`SceneComponent.K2_SetRelativeRotation` (`self.SM_Door`) (`KismetMathLibrary.RLerp` (struct) (`self.RotateDirection`) _newtrack_1) false false)
                      (set `self.IsDoorOpen` (not (`self.IsDoorOpen`)) :!label _label_2))))
                (:`<`
                  (set `self.RotateDirection` (struct :`Yaw` -90.0))
                  (goto _label))))
            (:`NewEnumerator1`
              ; Side-To-Side Transform Logic
              (bind (_direction_2 _newtrack_1_2) (`Timeline|Timeline_0` :!label _label_3)
                (:`Update`
                  (`SceneComponent.K2_SetRelativeTransform` (`self.SM_Door`) (`KismetMathLibrary.TLerp` (`KismetMathLibrary.MakeTransform` (0.0 59.0 0.0) (struct) (1.0 1.3 1.3)) (`KismetMathLibrary.MakeTransform` (0.0 176.0 0.0) (struct) (1.0 1.3 1.3)) _newtrack_1_2) false false)
                  (goto _label_2))))
            (:`NewEnumerator2`
              ; Up/Down Transform Logic
              (bind (_direction_3 _newtrack_1_3) (`Timeline|Timeline_1` :!label _label_4)
                (:`Update`
                  (`SceneComponent.K2_SetRelativeTransform` (`self.SM_Door`) (`KismetMathLibrary.TLerp` (`KismetMathLibrary.MakeTransform` (0.0 59.0 0.0) (struct) (1.0 1.3 1.3)) (`KismetMathLibrary.MakeTransform` (0.0 59.0 260.0) (struct) (1.0 1.3 1.3)) _newtrack_1_3) false false)
                  (goto _label_2))))))
        (:`B`
          (`BillboardComponent.SetSprite` _opendoorbillboardforward "/Game/Blueprints/T_OPEN.T_OPEN")
          (`BillboardComponent.SetSprite` (`self.OpenDoorBillboardBackward`) "/Game/Blueprints/T_OPEN.T_OPEN")
          (`AudioComponent.Play` (`self.PIXABAYdoor-open-close_CLOSE`) 0.0)
          (switch `/Game/Blueprints/ENums/E_DoorRotationType` (`self.RotateType`)
            (:`NewEnumerator0`
              (goto _label :!via `Reverse`))
            (:`NewEnumerator1`
              (goto _label_3 :!via `Reverse`))
            (:`NewEnumerator2`
              (goto _label_4 :!via `Reverse`))))))))

(event `/Game/Blueprints/BPI_Lock.Lock/Unlock`
  (bind _lockdoorbillboardforward (`self.LockDoorBillboardForward`))
  ;[1 1 1] Unlocks The Door
  (`AudioComponent.Play` (`self.PIXABAYlock-the-door`) 0.0)
  (bind _asbp_first_person_character (cast `/Game/FirstPerson/Blueprints/BP_FirstPersonCharacter` (`GameplayStatics.GetPlayerCharacter` 0)))
  (if (`/Game/FirstPerson/Blueprints/BP_FirstPersonCharacter.HasKey` _asbp_first_person_character)
    (if (`self.IsLocked`)
      (set `self.IsLocked` false)
      (`PrimitiveComponent.SetMaterial` (`self.SM_Door`) 0 "/Game/Materials/M_IncreaseHealth.M_IncreaseHealth")
      (`BillboardComponent.SetSprite` _lockdoorbillboardforward "/Game/Blueprints/T_LOCK.T_LOCK")
      (`BillboardComponent.SetSprite` (`self.LockDoorBillboardBackward`) "/Game/Blueprints/T_LOCK.T_LOCK")
      (else
        (set `self.IsLocked` true)
        (`PrimitiveComponent.SetMaterial` (`self.SM_Door`) 0 "/Game/Materials/M_ReduceHealth.M_ReduceHealth")
        (`BillboardComponent.SetSprite` _lockdoorbillboardforward "/Game/Blueprints/T_UNLOCK.T_UNLOCK")
        (`BillboardComponent.SetSprite` (`self.LockDoorBillboardBackward`) "/Game/Blueprints/T_UNLOCK.T_UNLOCK")))))

(event `/Game/Blueprints/BPI_TakeDamage.TakeDamage`
  (params (Amount :type "Float (double-precision)"))
  (bind _currenthealth (`self.CurrentHealth`))
  ; Applies damage to door
  (if (not (`self.IsDestroyed`))
    (bind _output_get (set `self.CurrentHealth` (- _currenthealth Amount)))
    (`KismetSystemLibrary.PrintString` (`KismetStringLibrary.Conv_DoubleToString` _currenthealth))
    (if (<= _output_get 0.0)
      ;; Destroys door component
      (`ActorComponent.K2_DestroyComponent` (`self.SM_Door`))
      (set `self.IsDestroyed` true)
      (`SceneComponent.SetVisibility` (`self.OpenDoorBillboardForward`) false false)
      (`SceneComponent.SetVisibility` (`self.OpenDoorBillboardBackward`) false false)
      (`SceneComponent.SetVisibility` (`self.LockDoorBillboardBackward`) false false)
      (`SceneComponent.SetVisibility` (`self.LockDoorBillboardForward`) false false))))

(event `self.CO_PlayerRangeCheckForward.OnComponentBeginOverlap`
  (params (OverlappedComponent :type "PrimitiveComponent Object Reference") (OtherActor :type "Actor Object Reference") (OtherComp :type "PrimitiveComponent Object Reference") (OtherBodyIndex :type Integer) (bFromSweep :type Boolean) (SweepResult :type "HitResult Structure (by ref)"))
  (bind _lockdoorbillboardforward (`self.LockDoorBillboardForward`))
  (if (`self.CheckBackwardActivated`)
    _
    (elif (not (`self.IsDestroyed`))
      (bind _asbp_first_person_character (cast `/Game/FirstPerson/Blueprints/BP_FirstPersonCharacter` OtherActor))
      (`SceneComponent.SetVisibility` (`self.OpenDoorBillboardForward`) true false)
      (`SceneComponent.SetVisibility` (`self.LockDoorBillboardForward`) true false)
      (if (`/Game/FirstPerson/Blueprints/BP_FirstPersonCharacter.HasKey` _asbp_first_person_character)
        (if (`self.IsLocked`)
          (`BillboardComponent.SetSprite` _lockdoorbillboardforward "/Game/Blueprints/T_UNLOCK.T_UNLOCK")
          (else
            (`BillboardComponent.SetSprite` _lockdoorbillboardforward "/Game/Blueprints/T_LOCK.T_LOCK")))
        (else
          (`BillboardComponent.SetSprite` (`self.LockDoorBillboardForward`) "/Game/Blueprints/T_NOKEY.T_NOKEY")))
      (set `self.CheckForwardActivated` true))))

(event `self.CO_PlayerRangeCheckForward.OnComponentEndOverlap`
  (params (OverlappedComponent :type "PrimitiveComponent Object Reference") (OtherActor :type "Actor Object Reference") (OtherComp :type "PrimitiveComponent Object Reference") (OtherBodyIndex :type Integer))
  (cast `/Game/FirstPerson/Blueprints/BP_FirstPersonCharacter` OtherActor)
  (`SceneComponent.SetVisibility` (`self.OpenDoorBillboardForward`) false false)
  (`SceneComponent.SetVisibility` (`self.LockDoorBillboardForward`) false false)
  (set `self.CheckForwardActivated` false))

(event `self.CO_PlayerRangeCheckBackward.OnComponentBeginOverlap`
  (params (OverlappedComponent :type "PrimitiveComponent Object Reference") (OtherActor :type "Actor Object Reference") (OtherComp :type "PrimitiveComponent Object Reference") (OtherBodyIndex :type Integer) (bFromSweep :type Boolean) (SweepResult :type "HitResult Structure (by ref)"))
  (bind _lockdoorbillboardbackward (`self.LockDoorBillboardBackward`))
  (if (`self.CheckForwardActivated`)
    _
    (elif (not (`self.IsDestroyed`))
      (bind _asbp_first_person_character (cast `/Game/FirstPerson/Blueprints/BP_FirstPersonCharacter` OtherActor))
      (`SceneComponent.SetVisibility` (`self.OpenDoorBillboardBackward`) true false)
      (`SceneComponent.SetVisibility` (`self.LockDoorBillboardBackward`) true false)
      (if (`/Game/FirstPerson/Blueprints/BP_FirstPersonCharacter.HasKey` _asbp_first_person_character)
        (if (`self.IsLocked`)
          (`BillboardComponent.SetSprite` _lockdoorbillboardbackward "/Game/Blueprints/T_UNLOCK.T_UNLOCK")
          (else
            (`BillboardComponent.SetSprite` _lockdoorbillboardbackward "/Game/Blueprints/T_LOCK.T_LOCK")))
        (else
          (`BillboardComponent.SetSprite` (`self.LockDoorBillboardBackward`) "/Game/Blueprints/T_NOKEY.T_NOKEY")))
      (set `self.CheckBackwardActivated` true))))

(event `self.CO_PlayerRangeCheckBackward.OnComponentEndOverlap`
  (params (OverlappedComponent :type "PrimitiveComponent Object Reference") (OtherActor :type "Actor Object Reference") (OtherComp :type "PrimitiveComponent Object Reference") (OtherBodyIndex :type Integer))
  (cast `/Game/FirstPerson/Blueprints/BP_FirstPersonCharacter` OtherActor)
  (`SceneComponent.SetVisibility` (`self.OpenDoorBillboardBackward`) false false)
  (`SceneComponent.SetVisibility` (`self.LockDoorBillboardBackward`) false false)
  (set `self.CheckBackwardActivated` false))

(fn `UserConstructionScript`
  (`|ExecutionSequence`
    (:`then_0`
      (if (`self.IsLocked`)
        (`PrimitiveComponent.SetMaterial` (`self.SM_Door`) 0 "/Game/Materials/M_ReduceHealth.M_ReduceHealth")
        (else
          (`PrimitiveComponent.SetMaterial` (`self.SM_Door`) 0 "/Game/Materials/M_IncreaseHealth.M_IncreaseHealth"))))
    (:`then_1`
      (if (`self.HasLight`)
        (`SceneComponent.SetVisibility` (`self.SM_DoorLightBox`) true false)
        (`SceneComponent.SetVisibility` (`self.DoorLight`) true false)
        (else
          (`SceneComponent.SetVisibility` (`self.SM_DoorLightBox`) false false)
          (`SceneComponent.SetVisibility` (`self.DoorLight`) false false))))
    (:`then_2`
      (switch `/Game/Blueprints/ENums/E_DoorType` (`self.DoorType`)
        (:`NewEnumerator0`
          (set `self.MaxHealth` 50.0)
          (set `self.DoorOpenSpeed` 2.0)
          (`PrimitiveComponent.SetMaterial` (`self.SM_Frame`) 0 "/Game/StarterContent/Materials/M_Wood_Oak.M_Wood_Oak"))
        (:`NewEnumerator1`
          (set `self.MaxHealth` 100.0)
          (set `self.DoorOpenSpeed` 1.0)
          (`PrimitiveComponent.SetMaterial` (`self.SM_Frame`) 0 "/Game/StarterContent/Props/Materials/M_Frame.M_Frame"))))))