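; Procedural dungeon generator actor that builds a chain of rooms at BeginPlay, starting with BP_Dungeon_Room_1 at its own transform.
; It keeps a pool of open exit points gathered from each room's ExitsFolder children.
; A recursive event removes a random exit and spawns a random RoomList class there, adding that room's exits until RoomAmount runs out.
; Rooms always spawn, with no overlap check.
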(event `self.ReceiveBeginPlay`
  (`self.SpawnStartRoom`)
  (`self.SpawnNextRoom`))

(event `SpawnStartRoom`
  ; Sapwn StartSRoom
  (bind _returnvalue (`|SpawnActorFromClass` "/Game/ProceduralDungeon/BP_Dungeon_Room_1.BP_Dungeon_Room_1_C" (`SceneComponent.K2_GetComponentToWorld` (`self.DefaultSceneRoot`)) "AlwaysSpawn" "MultiplyWithRoot" null null))
  (`KismetArrayLibrary.Array_Append` (`self.Exits List`) (`SceneComponent.GetChildrenComponents` (`/Game/ProceduralDungeon/BP_Master_Room.ExitsFolder` _returnvalue) false))
  (`KismetSystemLibrary.PrintString` "Hello"))

(event `SpawnNextRoom`
  (bind _selectedexitpoint (`self.SelectedExitPoint`))
  ; Spawn Next Room
  (bind _output_get (set `self.SelectedExitPoint` (`KismetArrayLibrary.Array_Random` (`self.Exits List`))))
  (`KismetArrayLibrary.Array_RemoveItem` (`self.Exits List`) _output_get)
  (bind _returnvalue (`|SpawnActorFromClass` (`KismetArrayLibrary.Array_Random` (`self.Room List`)) (`KismetMathLibrary.MakeTransform` (`SceneComponent.K2_GetComponentLocation` _selectedexitpoint) (`SceneComponent.K2_GetComponentRotation` _selectedexitpoint)) "AlwaysSpawn" "MultiplyWithRoot" null null))
  (bind _asbp_master_room (cast `/Game/ProceduralDungeon/BP_Master_Room` _returnvalue))
  (set `self.Latest Room` _asbp_master_room)
  (`KismetArrayLibrary.Array_Append` (`self.Exits List`) (`SceneComponent.GetChildrenComponents` (`/Game/ProceduralDungeon/BP_Master_Room.ExitsFolder` (`self.Latest Room`)) false))
  (bind _result (`/Engine/EditorBlueprintResources/StandardMacros.DecrementInt` (`self.Room Amount`))
    (:`  `
      (if (> _result 0)
        (`self.SpawnNextRoom`)))))

(fn `UserConstructionScript`)